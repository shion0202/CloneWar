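; BP_IRPlayerController is a player controller that reports player progress to online achievements and leaderboards.
; ClearStage1 and ClearStage10 events cache achievements, then write the matching stage-clear achievement.
; KillEnemy caches achievements, queries the KillEnemyAmount leaderboard stat, then writes it back incremented by one.
; Each step runs only on the preceding call's success, and BeginPlay, Tick and construction script do nothing.
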(event `self.ClearStage1`
  (`AchievementQueryCallbackProxy.CacheAchievements` self
    (:`OnSuccess`
      (`AchievementWriteCallbackProxy.WriteAchievementProgress` self "ACH_CLEAR_STAGE_1"))))

(event `self.ClearStage10`
  (`AchievementQueryCallbackProxy.CacheAchievements` self
    (:`OnSuccess`
      (`AchievementWriteCallbackProxy.WriteAchievementProgress` self "ACH_CLEAR_STAGE_10"))))

(event `self.KillEnemy`
  (`AchievementQueryCallbackProxy.CacheAchievements` self
    (:`OnSuccess`
      (bind _leaderboardvalue (`|LeaderboardQuery` self "KillEnemyAmount")
        (:`OnSuccess`
          (`LeaderboardBlueprintLibrary.WriteLeaderboardInteger` self "KillEnemyAmount" (+ _leaderboardvalue 1)))))))

(fn `UserConstructionScript`)