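; Shared Progressive UI helper functions for on-screen notifications and widget animation.
; Notify functions act only when player controller 0 is local, creating the WBP_PUI_Notify_Creator widget or forwarding small, large and bottom notifications to every top-level instance.
; Lerp helpers advance translation, scale, size or color one InterpTo step per call using world delta time.
; LerpBorderColor interpolates from ContentColorAndOpacity but writes BrushColor.
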(fn `Create notify system`
  (bind (_bool _controller) (`self.IsLocalControl` null))
  (if _bool
    (bind _returnvalue (`|CreateWidget` "/Game/ProgressiveUI/Blueprint/Notification/Notify/WBP_PUI_Notify_Creator.WBP_PUI_Notify_Creator_C" _controller))
    (`UserWidget.AddToViewport` _returnvalue 500)))

(fn `IsLocalControl`
  (returns (Bool :type Boolean) (Controller :type "PlayerController Object Reference"))
  (bind _returnvalue (`GameplayStatics.GetPlayerController` null))
  (return (`Controller.IsLocalPlayerController` _returnvalue) _returnvalue))

(fn `Lerp Border Color`
  (params (Border :type "Border Object Reference") (Color :type "LinearColor Structure" :default (struct :`R` 1.0 :`G` 1.0 :`B` 1.0 :`A` 1.0)) (Speed :type "Float (double-precision)" :default 8.0))
  (`Border.SetBrushColor` Border (`KismetMathLibrary.CInterpTo` (`Border.ContentColorAndOpacity` Border) Color (`GameplayStatics.GetWorldDeltaSeconds` null) Speed)))

(fn `Lerp Image Color`
  (params (Image :type "Image Object Reference") (Color :type "LinearColor Structure" :default (struct :`R` 1.0 :`G` 1.0 :`B` 1.0 :`A` 1.0)) (Speed :type "Float (double-precision)" :default 8.0))
  (`Image.SetColorAndOpacity` Image (`KismetMathLibrary.CInterpTo` (`Image.ColorAndOpacity` Image) Color (`GameplayStatics.GetWorldDeltaSeconds` null) Speed)))

(fn `Lerp Image Size`
  (params (Image :type "Image Object Reference") (Size :type "Vector2D Structure" :default (1.0 1.0)) (Speed :type "Float (double-precision)" :default 8.0))
  (`Image.SetBrushSize` Image (`KismetMathLibrary.Vector2DInterpTo` (`Widget.GetDesiredSize` Image) Size (`GameplayStatics.GetWorldDeltaSeconds` null) Speed)))

(fn `Lerp Sizebox Size`
  (params (`Size box` :type "SizeBox Object Reference") (Scale :type "Vector2D Structure" :default (30.0 30.0)) (Speed :type "Float (double-precision)" :default 8.0))
  (bind _returnvalue (`GameplayStatics.GetWorldDeltaSeconds` null))
  (bind (_x _y) (`KismetMathLibrary.BreakVector2D` Scale))
  (bind (_returnvalue_x _returnvalue_y) (`KismetMathLibrary.BreakVector2D` (`Widget.GetDesiredSize` `Size box`)))
  (`SizeBox.SetWidthOverride` `Size box` (`KismetMathLibrary.FInterpTo` _returnvalue_x _x _returnvalue Speed))
  (`SizeBox.SetHeightOverride` `Size box` (`KismetMathLibrary.FInterpTo` _returnvalue_y _y _returnvalue Speed)))

(fn `Lerp Text Color`
  (params (Text :type "TextBlock Object Reference") (Color :type "LinearColor Structure" :default (struct :`R` 1.0 :`G` 1.0 :`B` 1.0 :`A` 1.0)) (Speed :type "Float (double-precision)" :default 8.0))
  (bind (_colorandopacity_specifiedcolor _colorandopacity_coloruserule) (break `SlateColor` (`TextBlock.ColorAndOpacity` Text)))
  (`TextBlock.SetColorAndOpacity` Text (make `SlateColor` (`KismetMathLibrary.CInterpTo` _colorandopacity_specifiedcolor Color (`GameplayStatics.GetWorldDeltaSeconds` null) Speed) _colorandopacity_coloruserule)))

(fn `Lerp Widget Scale`
  (params (Widget :type "Widget Object Reference") (Scale :type "Vector2D Structure" :default (1.0 1.0)) (Speed :type "Float (double-precision)" :default 8.0))
  (bind (_rendertransform_translation _rendertransform_scale) (break `WidgetTransform` (`Widget.RenderTransform` Widget)))
  (`Widget.SetRenderScale` Widget (`KismetMathLibrary.Vector2DInterpTo` _rendertransform_scale Scale (`GameplayStatics.GetWorldDeltaSeconds` null) Speed)))

(fn `Lerp Widget Translation`
  (params (Widget :type "Widget Object Reference") (Pos :type "Vector2D Structure") (Speed :type "Float (double-precision)" :default 8.0))
  (bind _rendertransform_translation (break `WidgetTransform` (`Widget.RenderTransform` Widget)))
  (`Widget.SetRenderTranslation` Widget (`KismetMathLibrary.Vector2DInterpTo` _rendertransform_translation Pos (`GameplayStatics.GetWorldDeltaSeconds` null) Speed)))

(fn `Send bottom notify`
  (params (`Header text` :type Text) (`Body text` :type Text) (`Color head` :type "LinearColor Structure") (`Color body` :type "LinearColor Structure") (Delay :type "Float (double-precision)"))
  (if (`self.IsLocalControl` null)
    (bind _foundwidgets (`WidgetBlueprintLibrary.GetAllWidgetsOfClass` null "/Game/ProgressiveUI/Blueprint/Notification/Notify/WBP_PUI_Notify_Creator.WBP_PUI_Notify_Creator_C"))
    (for _array_element _foundwidgets
      (`/Game/ProgressiveUI/Blueprint/Notification/Notify/WBP_PUI_Notify_Creator.CreateNotify Bottom` _array_element `Color body` `Color head` `Header text` `Body text` Delay))))

(fn `Send large notify`
  (params (`Head text` :type Text) (`Description text` :type Text) (Icon :type "SlateBrush Structure") (`Color gradient` :type "LinearColor Structure") (`Color body` :type "LinearColor Structure") (Delay :type "Float (double-precision)"))
  (if (`self.IsLocalControl` null)
    (bind _foundwidgets (`WidgetBlueprintLibrary.GetAllWidgetsOfClass` null "/Game/ProgressiveUI/Blueprint/Notification/Notify/WBP_PUI_Notify_Creator.WBP_PUI_Notify_Creator_C"))
    (for _array_element _foundwidgets
      (`/Game/ProgressiveUI/Blueprint/Notification/Notify/WBP_PUI_Notify_Creator.CreateNotify Large` _array_element `Color body` `Color gradient` Icon `Head text` `Description text` Delay))))

(fn `Send small notify`
  (params (Text :type Text) (Icon :type "SlateBrush Structure") (`Color body` :type "LinearColor Structure") (`Color gradient` :type "LinearColor Structure") (`Delay time` :type "Float (double-precision)"))
  (if (`self.IsLocalControl` null)
    (bind _foundwidgets (`WidgetBlueprintLibrary.GetAllWidgetsOfClass` null "/Game/ProgressiveUI/Blueprint/Notification/Notify/WBP_PUI_Notify_Creator.WBP_PUI_Notify_Creator_C"))
    (for _array_element _foundwidgets
      (`/Game/ProgressiveUI/Blueprint/Notification/Notify/WBP_PUI_Notify_Creator.CreateNotify Small` _array_element `Color body` `Color gradient` Icon Text `Delay time`))))